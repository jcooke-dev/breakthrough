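; Brick3D_BP is a 3D brick for a Breakout-style game, with optional strong, unbreakable and extra-life variants.
; The construction script sets its color material from a map and shows the strength number, XXX mark or extra-life sprite.
; Ball hits reduce strength; destruction adds points and any extra life to the game instance, speeds up the ball and decrements the game state's bricks-to-clear count.
; Hit, destroy and extra-life outcomes play sounds.
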(event EventBeginPlay)

(event Collision|EventActorBeginOverlap
  (params (OtherActor :type Actor%20Object%20Reference)))

(event EventTick
  (params (DeltaSeconds :type Float%20%28single-precision%29)))

(event Collision|EventHit
  (params (MyComp :type Primitive%20Component%20Object%20Reference) (Other :type Actor%20Object%20Reference) (OtherComp :type Primitive%20Component%20Object%20Reference) (bSelfMoved :type Boolean) (HitLocation :type Vector :default "0, 0, 0") (HitNormal :type Vector :default "0, 0, 0") (NormalImpulse :type Vector :default "0, 0, 0") (Hit :type Hit%20Result%20Structure%20%28by%20ref%29))
  (bind _returnvalue (Actor|GetComponentbyClass Other "/Script/Engine.ProjectileMovementComponent"))
  ;[0.15 0.15 0.15 0.5] Reduce Strength from a Ball Hit and Take Other Actions, if Warranted: Destroy Brick, Gain an Extra Life, Update the Reduced Strength Mark, Add to Score, Increase the Ball Speed
  (if (Variables|Default|GetbIsUnbreakable)
    (Audio|PlaySound2D "/Game/sounds/wallHit_Cue.wallHit_Cue" 1.0 1.0 0.0 0 0)
    (elif (Class|GameplayStatics|ObjectIsA Other "/Game/Blueprints/Ball3D_BP.Ball3D_BP_C")
      (Variables|Default|SetnStrength (- (Variables|Default|GetnStrength) 1))
      (if (<= (Variables|Default|GetnStrength) 0)
        (bind _asgi_breakthrough (Utilities|Casting|CastToGI_Breakthrough (Game|GetGameInstance)))
        (if (Variables|Default|GetbIsExtraLife)
          (Variables|/Game/Blueprints/GI_Breakthrough.GI_Breakthrough_C|SetnNumLives _asgi_breakthrough (+ (Variables|/Game/Blueprints/GI_Breakthrough.GI_Breakthrough_C|GetnNumLives _asgi_breakthrough) 1))
          (Audio|PlaySound2D "/Game/sounds/extraLife_Cue.extraLife_Cue" 1.0 1.0 0.0 0 0))
        (Variables|/Game/Blueprints/GI_Breakthrough.GI_Breakthrough_C|SetnScore _asgi_breakthrough (+ (Variables|/Game/Blueprints/GI_Breakthrough.GI_Breakthrough_C|GetnScore _asgi_breakthrough) (Variables|Default|GetnPoints)))
        (bind _asgs_breakthrough (Utilities|Casting|CastToGS_Breakthrough (Game|GetGameState)))
        (Variables|/Game/Blueprints/GS_Breakthrough.GS_Breakthrough_C|SetfBallSpeed _asgs_breakthrough (+ (Math|Vector|VectorLength (Variables|/Script/Engine.MovementComponent|GetVelocity _returnvalue)) (Variables|/Game/Blueprints/GS_Breakthrough.GS_Breakthrough_C|GetfBallSpeedIncrement _asgs_breakthrough)))
        (Variables|/Script/Engine.MovementComponent|SetVelocity _returnvalue (* (Math|Vector|Normalize (Variables|/Script/Engine.MovementComponent|GetVelocity _returnvalue)) (+ (Math|Vector|VectorLength (Variables|/Script/Engine.MovementComponent|GetVelocity _returnvalue)) (Variables|/Game/Blueprints/GS_Breakthrough.GS_Breakthrough_C|GetfBallSpeedIncrement _asgs_breakthrough))))
        (Actor|DestroyActor)
        (if (Variables|Default|GetbIsStrong)
          (Audio|PlaySound2D "/Game/sounds/brickDestroy2_Cue.brickDestroy2_Cue" 1.0 1.0 0.0 0 0)
          (else
            (Audio|PlaySound2D "/Game/sounds/brickDestroy1_Cue.brickDestroy1_Cue" 1.0 1.0 0.0 0 0)))
        (bind _asgs_breakthrough_2 (Utilities|Casting|CastToGS_Breakthrough (Game|GetGameState)))
        (Variables|/Game/Blueprints/GS_Breakthrough.GS_Breakthrough_C|SetnNumBricksToClear _asgs_breakthrough_2 (- (Variables|/Game/Blueprints/GS_Breakthrough.GS_Breakthrough_C|GetnNumBricksToClear _asgs_breakthrough_2) 1))
        (else
          (Rendering|Components|TextRender|SetText (Variables|Default|GetPowerText) (Utilities|Text|ToText(String) (Variables|Default|GetnStrength)))
          (Audio|PlaySound2D "/Game/sounds/wallHit_Cue.wallHit_Cue" 1.0 1.0 0.0 0 0))))))

(fn ConstructionScript
  ;[0.15 0.15 0.15 0.5] Setting the Brick's Color (Sprite) and Marks/Decals (strength/life remaining number, unbreakable XXX, and extra life icon)
  (if (Variables|Default|GetbIsUnbreakable)
    (Variables|Default|SeteColor "NewEnumerator6"))
  (Rendering|Material|SetMaterial (Variables|Debug|GetStaticMeshComponent) 0 (.Value (Utilities|Map|Find (Variables|Default|GetmapColorMaterials) (Variables|Default|GeteColor))))
  (if (Variables|Default|GetbIsStrong)
    (Rendering|Components|TextRender|SetText (Variables|Default|GetPowerText) (Utilities|Text|ToText(String) (Variables|Default|GetnStrength))))
  (if (Variables|Default|GetbIsUnbreakable)
    (Rendering|Components|TextRender|SetText (Variables|Default|GetPowerText) (Utilities|Text|ToText(String) (Utilities|String|MakeLiteralString "XXX"))))
  (Rendering|SetVisibility (Variables|Default|GetPowerSprite) (Variables|Default|GetbIsExtraLife) false))