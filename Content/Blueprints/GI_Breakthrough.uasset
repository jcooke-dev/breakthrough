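; Game instance for Breakthrough that owns saved settings, persistent music and a shared lookup for the ball's movement.
; Init loads the settings save, creating one if absent, and Shutdown writes it back.
; BeginPlayingMusic runs once, applying the saved volume through a sound mix and spawning the chosen track to persist across levels.
; GetBallProjectileMovement finds the sprite or 3D ball's ProjectileMovementComponent, preferring 3D.
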(event EventInit
  (CallFunction|LoadGameSettings))

(event EventShutdown
  (CallFunction|SaveGameSettings))

(fn BeginPlayingMusic
  (bind _sgssettings (Variables|Default|GetsgsSettings))
  (if (not (Variables|Default|GetbMusicStarted))
    (Audio|PopSoundMixModifier "/Game/sounds/Music_Mix.Music_Mix")
    (Audio|SetSoundMixClassOverride "/Game/sounds/Music_Mix.Music_Mix" "/Game/sounds/Music.Music" (Variables|/Game/Blueprints/SaveGameSettings_BP.SaveGameSettings_BP_C|GetfMusicVol _sgssettings) 1.0 0.0 true)
    (Audio|PushSoundMixModifier "/Game/sounds/Music_Mix.Music_Mix")
    (bind _returnvalue (Audio|SpawnSound2D (.Value (Utilities|Map|Find (Variables|Default|GetmMusicTracks) (Variables|/Game/Blueprints/SaveGameSettings_BP.SaveGameSettings_BP_C|GetstrCurMusicTrack _sgssettings))) 1.0 1.0 0.0 0 true false))
    (Variables|Default|SetacMusic _returnvalue)
    (Variables|Default|SetbMusicStarted true)))

(fn LoadGameSettings
  (bind _strsettingssaveslot (Variables|Default|GetstrSettingsSaveSlot))
  (bind _returnvalue (SaveGame|LoadGamefromSlot _strsettingssaveslot))
  (bind _assave_game_settings_bp (Utilities|Casting|CastToSaveGameSettings_BP _returnvalue)
    (:then
      (Variables|Default|SetsgsSettings _assave_game_settings_bp))
    (:CastFailed
      (bind _returnvalue_2 (SaveGame|CreateSaveGameObject "/Game/Blueprints/SaveGameSettings_BP.SaveGameSettings_BP_C"))
      (bind _output_get (Variables|Default|SetsgsSettings _returnvalue_2))
      (SaveGame|SaveGametoSlot _output_get _strsettingssaveslot))))

(fn SaveGameSettings
  (SaveGame|SaveGametoSlot (Variables|Default|GetsgsSettings) (Variables|Default|GetstrSettingsSaveSlot)))

(fn GetBallProjectileMovement
  (Utilities|FlowControl|Sequence
    (:then_0
      (bind _returnvalue (Actor|GetActorOfClass "/Game/Blueprints/Ball_Sprite_BP.Ball_Sprite_BP_C"))
      (Utilities|IsValid _returnvalue
        (:Is%20Valid
          (Variables|Default|SetoBallProjMoveComp (Actor|GetComponentbyClass _returnvalue "/Script/Engine.ProjectileMovementComponent")))))
    (:then_1
      (bind _returnvalue_2 (Actor|GetActorOfClass "/Game/Blueprints/Ball3D_BP.Ball3D_BP_C"))
      (Utilities|IsValid _returnvalue_2
        (:Is%20Valid
          (Variables|Default|SetoBallProjMoveComp (Actor|GetComponentbyClass _returnvalue_2 "/Script/Engine.ProjectileMovementComponent")))))
    (:then_2
      (return (Variables|Default|GetoBallProjMoveComp)))))