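; Player controller for a Breakthrough game that handles autoplay toggling, pause and quit, and paddle input detection.
; Ctrl+A flips AutoPlay on the game state, while Escape branches on its EGameState to quit from the main menu or toggle pause.
; Pausing lazily creates and shows a Paused widget and switches cursor and input mode.
; Tick sets paddle direction from Left/Right keys, with horizontal mouse movement clearing the keyboard-control flag.
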(event EventTick
  (params (DeltaSeconds :type Float%20%28single-precision%29))
  (if (> (Math|Float|Absolute(Float) (.DeltaX (Class|PlayerController|GetInputMouseDelta))) 0.0)
    (Variables|Default|SetbPadMoveByKeys false))
  (if (Game|Player|IsInputKeyDown "Left")
    (Variables|Default|SetfPadMovePolarity -1.0)
    (Variables|Default|SetbPadMoveByKeys true :!label _label)
    (elif (Game|Player|IsInputKeyDown "Right")
      (Variables|Default|SetfPadMovePolarity 1.0)
      (goto _label)
      (else
        (Variables|Default|SetfPadMovePolarity 0.0)))))

(event Input|KeyboardEvents|Escape
  (params (Key :type Key%20Structure :default "None"))
  (bind _returnvalue (Game|GetPlayerController 0))
  (bind _returnvalue_2 (Game|GetPlayerController 0))
  (:Pressed
    (bind _asgs_breakthrough (Utilities|Casting|CastToGS_Breakthrough (Game|GetGameState)))
    (switch Utilities|FlowControl|Switch|SwitchoneGameState (Variables|/Game/Blueprints/GS_Breakthrough.GS_Breakthrough_C|GeteGameState _asgs_breakthrough)
      (:NewEnumerator0
        (Game|QuitGame 0 "Quit" false))
      (:NewEnumerator1
        (Utilities|IsValid (Variables|Default|GetwPaused)
          (:Is%20Valid
            _)
          (:Is%20Not%20Valid
            (bind _returnvalue_3 (UserInterface|CreateWidget "/Game/UI/Paused.Paused_C"))
            (Variables|Default|SetwPaused _returnvalue_3)))
        (UserInterface|Viewport|AddtoViewport (Variables|Default|GetwPaused) 0)
        (Game|SetGamePaused true)
        (Variables|/Script/Engine.PlayerController|SetbShowMouseCursor _returnvalue true)
        (Input|SetInputModeGameandUI _returnvalue 0 "DoNotLock" true false)
        (bind _asgs_breakthrough_2 (Utilities|Casting|CastToGS_Breakthrough (Game|GetGameState)))
        (Variables|/Game/Blueprints/GS_Breakthrough.GS_Breakthrough_C|SeteGameState _asgs_breakthrough_2 "NewEnumerator2"))
      (:NewEnumerator2
        (Game|SetGamePaused false)
        (Variables|/Script/Engine.PlayerController|SetbShowMouseCursor _returnvalue_2 false)
        (Input|SetInputModeGameOnly _returnvalue_2 false)
        (Widget|RemovefromParent (Variables|Default|GetwPaused))
        (bind _asgs_breakthrough_3 (Utilities|Casting|CastToGS_Breakthrough (Game|GetGameState)))
        (Variables|/Game/Blueprints/GS_Breakthrough.GS_Breakthrough_C|SeteGameState _asgs_breakthrough_3 "NewEnumerator1")))))

(event Input|KeyboardEvents|CtrlA
  (params (Key :type Key%20Structure :default "None"))
  (:Pressed
    (bind _asgs_breakthrough (Utilities|Casting|CastToGS_Breakthrough (Game|GetGameState)))
    (Variables|/Game/Blueprints/GS_Breakthrough.GS_Breakthrough_C|SetbAutoPlay _asgs_breakthrough (not (Variables|/Game/Blueprints/GS_Breakthrough.GS_Breakthrough_C|GetbAutoPlay _asgs_breakthrough)))))

(fn ConstructionScript)