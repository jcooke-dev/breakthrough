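; Ball actor Blueprint, apparently sprite-based by its name, with a ProjectileMovement component and no active graph logic.
; All script nodes are disabled, unconnected or unused, leaving any motion to component settings outside the graph.
; The leftovers sketch hand-written movement: position integrated from velocity, swept location updates, hit impulses added to velocity and a Z-flip bounce.
; Disabled debug prints show velocity and hit impulse.
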(event EventTick
  (params (DeltaSeconds :type Float%20%28single-precision%29))
  (Development|PrintString (Utilities|String|ToString(Vector) (Variables|/Script/Engine.MovementComponent|GetVelocity (Variables|Default|GetProjectileMovement)))))

(event Collision|EventHit
  (params (MyComp :type Primitive%20Component%20Object%20Reference) (Other :type Actor%20Object%20Reference) (OtherComp :type Primitive%20Component%20Object%20Reference) (bSelfMoved :type Boolean) (HitLocation :type Vector :default "0, 0, 0") (HitNormal :type Vector :default "0, 0, 0") (NormalImpulse :type Vector :default "0, 0, 0") (Hit :type Hit%20Result%20Structure%20%28by%20ref%29))
  (Development|PrintString (Utilities|String|ToString(Vector) NormalImpulse))
  (Variables|Default|SetvVel (+ (* NormalImpulse 1.5e+02) (Variables|Default|GetvVel))))

(event EventBeginPlay
  (Variables|Default|SetvPos "-150.000000,0.000000,250.000000")
  (Variables|Default|SetvVel "50.000000,0.000000,-300.000000"))

(fn ConstructionScript)