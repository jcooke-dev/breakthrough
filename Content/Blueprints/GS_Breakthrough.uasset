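; Game state for the Breakthrough brick-clearing game, managing the HUD and detecting level completion.
; Creates the HUD and fires a viewport-resized dispatcher on size changes and once the tilemap projects on screen, so HUD offsets can follow that actor.
; Each tick checks remaining bricks; at zero it updates the GameInstance state, plays a level-name-dependent camera shake, then shows a level-cleared popup after a short delay.
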(event EventBeginPlay
  (bind _returnvalue (Viewport|GetViewportSize))
  (bind _returnvalue_2 (UserInterface|CreateWidget "/Game/UI/HUD.HUD_C"))
  (Variables|Default|SetwHUD _returnvalue_2)
  (Variables|Default|SetvLastViewportSize _returnvalue)
  (Variables|Default|SetvCurViewportSize _returnvalue)
  (Default|CallEvDisViewportResized))

(event EventTick
  (params (DeltaSeconds :type Float%20%28single-precision%29))
  (bind _returnvalue (Game|GetPlayerController 0))
  (bind _returnvalue_2 (Viewport|GetViewportSize))
  (bind (_x _y) (Math|Vector2D|BreakVector2D _returnvalue_2))
  (Utilities|FlowControl|Sequence
    (:then_0
      (if (Variables|Default|GetbTileMapOnScreen)
        ;[0.15 0.15 0.15 0.5] Detect Viewport Size Changes and Call the Custom Event to Adjust the HUD Widget's Offsets
        (bind _output_get (Variables|Default|SetvCurViewportSize (Viewport|GetViewportSize)))
        (if (Class|KismetMathLibrary|NotEqualExactlyVector2DVector2D (Variables|Default|GetvLastViewportSize) _output_get)
          (Default|CallEvDisViewportResized)
          (Variables|Default|SetvLastViewportSize _output_get))
        (else
          ;[0.15 0.15 0.15 0.5] Check that the TileMap is Actually OnScreen (Needed Since the HUD Widget Offset is Based on this Actor's Position) - If so, Call the Viewport Resized Event
          (bind _returnvalue_3 (Actor|GetActorOfClass "/Script/Paper2D.PaperTileMapActor"))
          (Utilities|IsValid _returnvalue_3
            (:Is%20Valid
              (bind _output_get_2 (Variables|Default|SetbTileMapOnScreen (Math|Boolean|ANDBoolean (> (.X (Math|Vector2D|BreakVector2D (.ScreenPosition (Class|WidgetLayoutLibrary|ProjectWorldLocationtoWidgetPosition (Game|GetPlayerController 0) (Transformation|GetActorLocation _returnvalue_3) false)))) 0.0) (> (.Y (Math|Vector2D|BreakVector2D (.ScreenPosition (Class|WidgetLayoutLibrary|ProjectWorldLocationtoWidgetPosition (Game|GetPlayerController 0) (Transformation|GetActorLocation _returnvalue_3) false)))) 0.0) (< (.X (Math|Vector2D|BreakVector2D (.ScreenPosition (Class|WidgetLayoutLibrary|ProjectWorldLocationtoWidgetPosition (Game|GetPlayerController 0) (Transformation|GetActorLocation _returnvalue_3) false)))) _x) (< (.Y (Math|Vector2D|BreakVector2D (.ScreenPosition (Class|WidgetLayoutLibrary|ProjectWorldLocationtoWidgetPosition (Game|GetPlayerController 0) (Transformation|GetActorLocation _returnvalue_3) false)))) _y))))
              (if _output_get_2
                (Default|CallEvDisViewportResized)))))))
    (:then_1
      ;[0.15 0.15 0.15 0.5] Have All Bricks been Cleared from this Level?
      (bind _asgi_breakthrough (Utilities|Casting|CastToGI_Breakthrough (Game|GetGameInstance)))
      (if (Utilities|Enum|Equal(Enum) (Variables|/Game/Blueprints/GI_Breakthrough.GI_Breakthrough_C|GeteGameState _asgi_breakthrough) "NewEnumerator1")
        (if (<= (Variables|Default|GetnNumBricksToClear) 0)
          (Variables|/Game/Blueprints/GI_Breakthrough.GI_Breakthrough_C|SeteGameState _asgi_breakthrough "NewEnumerator4")
          (bind _returnvalue_4 (Game|GetCurrentLevelName true))
          (if (Utilities|String|Contains _returnvalue_4 "GameplayLevel")
            (Game|Feedback|ClientStartCameraShake _returnvalue "/Game/Blueprints/CamShake_LevelCleared_2D_BP.CamShake_LevelCleared_2D_BP_C" 1.0 "CameraLocal" "0, 0, 0")
            (else
              (Game|Feedback|ClientStartCameraShake _returnvalue "/Game/Blueprints/CamShake_LevelCleared_BP.CamShake_LevelCleared_BP_C" 1.0 "CameraLocal" "0, 0, 0")))
          (Utilities|FlowControl|Delay 1.0)
          (Utilities|IsValid (Variables|Default|GetwLevelCleared)
            (:Is%20Valid
              _)
            (:Is%20Not%20Valid
              (bind _returnvalue_5 (UserInterface|CreateWidget "/Game/UI/PopUpMenu.PopUpMenu_C" 0 "NewEnumerator2"))
              (Variables|Default|SetwLevelCleared _returnvalue_5)))
          (UserInterface|Viewport|AddtoViewport (Variables|Default|GetwLevelCleared) 0))))))

(fn ConstructionScript)