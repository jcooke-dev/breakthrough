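; Ball actor for the Breakthrough game, riding with the paddle before launch and bouncing around the level.
; Construction sets projectile speed from the game state and picks a mesh material from the game instance's theme.
; While in launch mode, Tick sweeps the ball to the X position of the sprite or 3D paddle.
; Hit events play separate sounds for paddle and tile-map wall impacts.
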(event EventBeginPlay)

(event Collision|EventHit
  (params (MyComp :type Primitive%20Component%20Object%20Reference) (Other :type Actor%20Object%20Reference) (OtherComp :type Primitive%20Component%20Object%20Reference) (bSelfMoved :type Boolean) (HitLocation :type Vector :default "0, 0, 0") (HitNormal :type Vector :default "0, 0, 0") (NormalImpulse :type Vector :default "0, 0, 0") (Hit :type Hit%20Result%20Structure%20%28by%20ref%29))
  (Utilities|FlowControl|Sequence
    (:then_0
      (if (or (Class|GameplayStatics|ObjectIsA Other "/Game/Blueprints/Paddle_Sprite_BP.Paddle_Sprite_BP_C") (Class|GameplayStatics|ObjectIsA Other "/Game/Blueprints/Paddle3D_BP.Paddle3D_BP_C"))
        (Audio|PlaySound2D "/Game/sounds/paddleHit_Cue.paddleHit_Cue" 1.0 1.0 0.0 0 0)))
    (:then_1
      (if (Class|GameplayStatics|ObjectIsA Other "/Script/Paper2D.PaperTileMapActor")
        (Audio|PlaySound2D "/Game/sounds/wallHit_Cue.wallHit_Cue" 1.0 1.0 0.0 0 0)))))

(event EventTick
  (params (DeltaSeconds :type Float%20%28single-precision%29))
  (bind _returnvalue (Transformation|GetActorLocation))
  (bind (_x _y _z) (Math|Vector|BreakVector _returnvalue))
  ;[0.15 0.15 0.15 0.5] Match the Ball's Position to the Paddle's, if in LAUNCH mode
  (bind _asgi_breakthrough (Utilities|Casting|CastToGI_Breakthrough (Game|GetGameInstance)))
  (if (Utilities|Enum|Equal(Enum) (Variables|/Game/Blueprints/GI_Breakthrough.GI_Breakthrough_C|GeteGameState _asgi_breakthrough) "NewEnumerator3")
    (CallFunction|UpdatePaddlePos)
    (Transformation|SetActorLocation (Math|Vector|MakeVector (.X (Math|Vector|BreakVector (Variables|Default|GetvPaddlePos))) _y _z) true false)))

(fn ConstructionScript
  (bind _asgs_breakthrough (Utilities|Casting|CastToGS_Breakthrough (Game|GetGameState)))
  (Variables|/Script/Engine.ProjectileMovementComponent|SetInitialSpeed (Variables|Default|GetProjectileMovement) (Variables|/Game/Blueprints/GS_Breakthrough.GS_Breakthrough_C|GetfBallSpeed _asgs_breakthrough))
  (bind _asgi_breakthrough (Utilities|Casting|CastToGI_Breakthrough (Game|GetGameInstance)))
  (Rendering|Material|SetMaterial (Variables|Debug|GetStaticMeshComponent) 0 (.Value (Utilities|Map|Find (Variables|Default|GetmapMaterials) (Variables|/Game/Blueprints/GI_Breakthrough.GI_Breakthrough_C|GeteTheme _asgi_breakthrough)))))

(fn UpdatePaddlePos
  (Utilities|FlowControl|Sequence
    (:then_0
      (bind _returnvalue (Actor|GetActorOfClass "/Game/Blueprints/Paddle_Sprite_BP.Paddle_Sprite_BP_C"))
      (Utilities|IsValid _returnvalue
        (:Is%20Valid
          (Variables|Default|SetvPaddlePos (Transformation|GetActorLocation _returnvalue)))))
    (:then_1
      (bind _returnvalue_2 (Actor|GetActorOfClass "/Game/Blueprints/Paddle3D_BP.Paddle3D_BP_C"))
      (Utilities|IsValid _returnvalue_2
        (:Is%20Valid
          (Variables|Default|SetvPaddlePos (Transformation|GetActorLocation _returnvalue_2)))))))