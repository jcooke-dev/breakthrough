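; RollingAvg_Float_BP is a utility that keeps a rolling average over the most recent float samples, up to a set capacity.
; AddValue appends to an array until it is full, then shifts every element down one slot and writes the new value last, dropping the oldest.
; GetAverage sums the stored values and divides by the current count, guarding against division by zero and returning zero when empty.
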(fn AddValue
  (params (fValue :type Float%20%28double-precision%29))
  (bind _arelements (Variables|Default|GetarElements))
  (bind _arelements_2 (Variables|Default|GetarElements))
  (if (== (Variables|Default|GetnSize) (Variables|Default|GetnCapacity))
    (for _index (range 0 (- (Variables|Default|GetnCapacity) 2))
      (Utilities|Array|SetArrayElem _arelements_2 _index (Utilities|Array|Get(acopy) _arelements_2 (+ _index 1))))
    (Utilities|Array|SetArrayElem _arelements (- (Variables|Default|GetnSize) 1) fValue)
    (else
      (Utilities|Array|Add _arelements fValue)
      (Math|Integer|IncrementInt (Variables|Default|GetnSize)))))

(fn GetAverage
  (bind _nsize (Variables|Default|GetnSize))
  (for _array_element (Variables|Default|GetarElements)
    (LocalVariables|SetfSum (+ _array_element (LocalVariables|GetfSum))))
  (return (Math|Float|SelectFloat (/ (LocalVariables|GetfSum) (Math|Integer|SelectInt _nsize 1 (!= _nsize 0))) 0.0 (> (Variables|Default|GetnSize) 0))))