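; Geometry collection actor for a chamfered brick block that shatters as soon as play begins, then removes itself.
; BeginPlay fires a radial impulse with strain at the component's location, randomly shifted in X and Z so each fracture looks different.
; The actor destroys itself after a configurable delay.
; The construction script applies a configurable material to the collection's first slot.
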(event EventBeginPlay
  (bind _returnvalue (Math|Float|MakeLiteralFloat 3.8e+02))
  (bind _returnvalue_2 (Math|Float|MakeLiteralFloat 3e+02))
  (bind _geometrycollectioncomponent (Variables|Default|GetGeometryCollectionComponent))
  (bind _returnvalue_3 (Transformation|GetWorldLocation _geometrycollectioncomponent))
  (bind (_x _y _z) (Math|Vector|BreakVector _returnvalue_3))
  (Class|PhysicsObjectBlueprintLibrary|ApplyRadialImpulse (Variables|Default|GetGeometryCollectionComponent) (Math|Vector|MakeVector (+ _x (- (/ _returnvalue_2 2.0) (* _returnvalue_2 (Math|Random|RandomFloat)))) _y (+ _z (- (/ _returnvalue 2.0) (* _returnvalue (Math|Random|RandomFloat))))) 5e+02 1.5e+04 "RIF_Constant" true 1e+03 false 0.0 1.0)
  (Utilities|FlowControl|Delay (Variables|Default|GetfTimeToDestroy))
  (Actor|DestroyActor))

(fn ConstructionScript
  (Rendering|Material|SetMaterial (Variables|Default|GetGeometryCollectionComponent) 0 (Variables|Default|GetmiMaterial)))