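; Brick actor for a Breakthrough-style ball-and-brick game, with variants for strong, unbreakable and extra-life bricks.
; The construction script picks the sprite from a color map, shows strength or "XXX" as text, and toggles the extra-life sprite.
; Ball hits lower the strength of breakable bricks, updating the text until it reaches zero.
; The destroyed brick then adds points and any extra life to GS_Breakthrough and slightly speeds up the ball.
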(event EventBeginPlay)

(event Collision|EventActorBeginOverlap
  (params (OtherActor :type Actor%20Object%20Reference)))

(event EventTick
  (params (DeltaSeconds :type Float%20%28single-precision%29)))

(event Collision|EventHit
  (params (MyComp :type Primitive%20Component%20Object%20Reference) (Other :type Actor%20Object%20Reference) (OtherComp :type Primitive%20Component%20Object%20Reference) (bSelfMoved :type Boolean) (HitLocation :type Vector :default "0, 0, 0") (HitNormal :type Vector :default "0, 0, 0") (NormalImpulse :type Vector :default "0, 0, 0") (Hit :type Hit%20Result%20Structure%20%28by%20ref%29))
  (bind _returnvalue (Actor|GetComponentbyClass Other "/Script/Engine.ProjectileMovementComponent"))
  ;[0.15 0.15 0.15 0.5] Reduce Strength and Destroy Brick?
  (if (not (Variables|Default|GetbIsUnbreakable))
    (if (Class|GameplayStatics|ObjectIsA Other "/Game/Blueprints/Ball_Sprite_Blueprint.Ball_Sprite_Blueprint_C")
      (Variables|Default|SetnStrength (- (Variables|Default|GetnStrength) 1))
      (if (<= (Variables|Default|GetnStrength) 0)
        (bind _asgs_breakthrough (Utilities|Casting|CastToGS_Breakthrough (Game|GetGameState)))
        (if (Variables|Default|GetbIsExtraLife)
          (Variables|/Game/Blueprints/GS_Breakthrough.GS_Breakthrough_C|SetnNumLives _asgs_breakthrough (+ (Variables|/Game/Blueprints/GS_Breakthrough.GS_Breakthrough_C|GetnNumLives _asgs_breakthrough) 1)))
        (Variables|/Game/Blueprints/GS_Breakthrough.GS_Breakthrough_C|SetnScore _asgs_breakthrough (+ (Variables|/Game/Blueprints/GS_Breakthrough.GS_Breakthrough_C|GetnScore _asgs_breakthrough) (Variables|Default|GetnPoints)))
        (Variables|/Script/Engine.MovementComponent|SetVelocity _returnvalue (* (Math|Vector|Normalize (Variables|/Script/Engine.MovementComponent|GetVelocity _returnvalue)) (+ (Math|Vector|VectorLength (Variables|/Script/Engine.MovementComponent|GetVelocity _returnvalue)) 5.0)))
        (Actor|DestroyActor)
        (else
          (Rendering|Components|TextRender|SetText (Variables|Default|GetPowerText) (Utilities|Text|ToText(String) (Variables|Default|GetnStrength))))))))

(fn ConstructionScript
  ;[0.15 0.15 0.15 0.5] Setting the Brick's Color (Sprite)
  (if (Variables|Default|GetbIsUnbreakable)
    (Variables|Default|SeteColor "NewEnumerator6"))
  (Rendering|Components|Sprite|SetSprite (Variables|Default|GetRenderComponent) (.Value (Utilities|Map|Find (Variables|Default|GetmapColorsSprites) (Variables|Default|GeteColor))))
  (if (Variables|Default|GetbIsStrong)
    (Rendering|Components|TextRender|SetText (Variables|Default|GetPowerText) (Utilities|Text|ToText(String) (Variables|Default|GetnStrength))))
  (if (Variables|Default|GetbIsUnbreakable)
    (Rendering|Components|TextRender|SetText (Variables|Default|GetPowerText) (Utilities|Text|ToText(String) (Utilities|String|MakeLiteralString "XXX"))))
  (Rendering|SetVisibility (Variables|Default|GetPowerSprite) (Variables|Default|GetbIsExtraLife) false))