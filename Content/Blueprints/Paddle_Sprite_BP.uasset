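; Player paddle for a Breakout-style game, moved only along the X axis with swept location updates every Tick.
; When the game state's AutoPlay flag is on, it copies the ball's X, skipping frames with no valid ball.
; Otherwise the player controller selects either key movement, scaled by polarity, speed and delta time, or mouse movement, which sets X directly from the viewport cursor position.
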(event EventTick
  (params (DeltaSeconds :type Float%20%28single-precision%29))
  (bind _returnvalue (Transformation|GetActorLocation))
  (bind _returnvalue_2 (Transformation|GetActorLocation))
  (bind _returnvalue_3 (Transformation|GetActorLocation))
  (bind _returnvalue_4 (Class|WidgetLayoutLibrary|GetViewportScale))
  (bind _returnvalue_5 (Viewport|GetViewportSize))
  (bind (_x _y _z) (Math|Vector|BreakVector _returnvalue))
  (bind (_x_2 _y_2 _z_2) (Math|Vector|BreakVector _returnvalue_2))
  (bind _x_3 (Math|Vector2D|BreakVector2D _returnvalue_5))
  (bind (_x_4 _y_3 _z_3) (Math|Vector|BreakVector _returnvalue_3))
  ;[0.15 0.15 0.15 0.5] Moving Paddle by Keys, Mouse, or AutoPlay?
  (bind _asplayer_controller_bp (Utilities|Casting|CastToPlayerController_BP (Game|GetPlayerController 0)))
  (bind _asgs_breakthrough (Utilities|Casting|CastToGS_Breakthrough (Game|GetGameState)))
  (if (Variables|/Game/Blueprints/GS_Breakthrough.GS_Breakthrough_C|GetbAutoPlay _asgs_breakthrough)
    ;[0.15 0.15 0.15 0.5] AutoPlay Movement
    (bind _returnvalue_6 (Actor|GetActorOfClass "/Game/Blueprints/Ball_Sprite_BP.Ball_Sprite_BP_C"))
    (Utilities|IsValid _returnvalue_6 ; this ensures a valid ball before referencing (can happen if AutoPlay engaged during ball destruction and spawn - non-zero lives
      (:Is%20Valid
        (Transformation|SetActorLocation (Math|Vector|MakeVector (.X (Math|Vector|BreakVector (Transformation|GetActorLocation _returnvalue_6))) _y_3 _z_3) true false)))
    (elif (Variables|/Game/Blueprints/PlayerController_BP.PlayerController_BP_C|GetbPadMoveByKeys _asplayer_controller_bp)
      ;[0.15 0.15 0.15 0.5] Key Movement
      (Transformation|SetActorLocation (Math|Vector|MakeVector (+ (* (Variables|/Game/Blueprints/PlayerController_BP.PlayerController_BP_C|GetfPadMovePolarity _asplayer_controller_bp) (* DeltaSeconds (Variables|Default|GetfPaddleSpeed))) _x) _y _z) true false)
      (else
        ;[0.15 0.15 0.15 0.5] Mouse Movement
        (bind _returnvalue_7 (Class|WidgetLayoutLibrary|GetMousePositiononViewport))
        (Transformation|SetActorLocation (Math|Vector|MakeVector (/ (* (/ (* _returnvalue_4 (.X (Math|Vector2D|BreakVector2D _returnvalue_7))) _x_3) _x_3) _returnvalue_4) _y_2 _z_2) true false)))))

(fn ConstructionScript)